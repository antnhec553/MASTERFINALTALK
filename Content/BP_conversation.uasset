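; BP_conversation is a dialogue Blueprint that shows lines from a Dialogue array in a BPW_Textual widget.
; Each Talk event increments Talkindex, then either creates the widget and adds it to the viewport or updates its text if it already exists.
; The creation call sets no text, and the array-length check is unconnected, so the widget-removal branch never runs.
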(event EventBeginPlay)

(event Collision|EventActorBeginOverlap
  (params (OtherActor :type Actor%20Object%20Reference)))

(event EventTick
  (params (DeltaSeconds :type Float%20%28single-precision%29)))

(event EventTalk
  (Math|Integer|IncrementInt (Variables|Default|Gettalkindex)
    (:%20%20
      (if true
        (Variables|Default|Getui
          (:then
            (Rendering|Components|TextRender|SetText (Variables|/Game/ThirdPerson/Blueprints/BPW_Textual.BPW_Textual_C|Gettext (Variables|Default|Getui)) (Utilities|Text|ToText(String) (Utilities|Array|Get(acopy) (Variables|Default|GetDialogue) (Variables|Default|Gettalkindex)))))
          (:else
            (bind _returnvalue (UserInterface|CreateWidget "/Game/ThirdPerson/Blueprints/BPW_Textual.BPW_Textual_C" (Game|GetPlayerController 0)))
            (bind _output_get (Variables|Default|Setui _returnvalue))
            (UserInterface|Viewport|AddtoViewport _output_get 0)))
        (else
          (Widget|RemovefromParent (Variables|Default|Getui)))))))

(fn ConstructionScript)